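; BP_ShowTestUI is a debug helper Blueprint for toggling a test UI and inspecting player pawn state.
; ShowTestUI creates WB_ThielMainUI at a high viewport Z-order, or removes and clears it if already present.
; PrintPawnState prints the player character's PawnStateComponent as a string.
; StartPhysUpdate and StopPhysUpdate pass true or false to SetPhysUpdate, which has an empty body here.
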(fn `PrintPawnState`
  (`KismetSystemLibrary.PrintString` (`PawnStateComponent.ToString` (`Actor.GetComponentByClass` (`GameplayStatics.GetPlayerCharacter` 0) "/Script/PawnState.PawnStateComponent"))))

(fn `SetPhysUpdate`
  (params (Enabled :type Boolean))
  (locals (NeedUpdate :type Boolean)))

(fn `ShowTestUI`
  (bind _testui (`self.TestUI`)
    (:`then`
      (`Widget.RemoveFromParent` _testui)
      (set `self.TestUI` null))
    (:`else`
      (bind _returnvalue (`|CreateWidget` "/Game/Sandbox/Thielzhang/UI/WB_ThielMainUI.WB_ThielMainUI_C"))
      (bind _output_get (set `self.TestUI` _returnvalue))
      (`UserWidget.AddToViewport` _output_get 100))))

(fn `StartPhysUpdate`
  (`self.SetPhysUpdate` true))

(fn `StopPhysUpdate`
  (`self.SetPhysUpdate` false))