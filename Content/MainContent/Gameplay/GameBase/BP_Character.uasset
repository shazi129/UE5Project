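; Game base character Blueprint that serves as a test harness for RPCs.
; Pressing E fires ServerTestRPC, which calls TestRPC and spawns a BP_BillboardActor at a fixed transform.
; TestRPC casts the first actor tagged RPCActor to BP_TestRPCActor and calls StartServerTest on its TestRPC member.
; BeginPlay loops over the GameFeatures AutoActivate config array with an empty body, so it activates nothing.
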(event `self.ReceiveBeginPlay`
  (for _ (`GameplayBPLibrary.GetArrayGameplayConfig` "GameFeatures" "AutoActivate")
    _))

(event `self.ReceiveEndPlay`
  (params (EndPlayReason :type "EEndPlayReason Enum" :default "Destroyed")))

(event `Key|E`
  (params (Key :type "Key Structure"))
  (:`Pressed`
    (`self.ServerTestRPC`)))

(event `ServerTestRPC`
  (`self.TestRPC`)
  (`|SpawnActorFromClass` "/Game/MainContent/TestContent/BillBoard/BP_BillboardActor.BP_BillboardActor_C" (`KismetMathLibrary.MakeTransform` (100.0 100.0 210.0)) "AlwaysSpawn" "OverrideRootScale" null null))

(fn `TestRPC`
  (bind _outactors (`GameplayStatics.GetAllActorsWithTag` "RPCActor"))
  (if (> (`KismetArrayLibrary.Array_Length` _outactors) 0)
    (bind _asbp_test_rpcactor (cast `/Game/MainContent/TestContent/RPC/BP_TestRPCActor` (`|GetArrayItem` _outactors)))
    (`TestRPCComponent.StartServerTest` (`/Game/MainContent/TestContent/RPC/BP_TestRPCActor.TestRPC` _asbp_test_rpcactor))))

(fn `UserConstructionScript`)