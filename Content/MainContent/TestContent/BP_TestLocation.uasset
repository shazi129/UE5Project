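; BP_TestLocation is a test Blueprint for debug printing and trying out graph features.
; On BeginPlay it prints a separator and the Cube component's relative location.
; TestEditorFunc prints the result of IsRunning, and a custom event passes its parameter into the collapsed Test Collapse graph, which plays a timeline and outputs false on update.
; The construction script and NewFunction_0 are empty.
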(event `self.ReceiveBeginPlay`
  (`KismetSystemLibrary.PrintString` "======================")
  (`KismetSystemLibrary.PrintString` (`KismetStringLibrary.Conv_Vector3fToString` (`SceneComponent.RelativeLocation` (`self.Cube`)))))

(event `TestEditorFunc`
  (`KismetSystemLibrary.PrintString` (`KismetStringLibrary.Conv_BoolToString` (`ExGameplayLibrary.IsRunning` null))))

(event `CustomEvent_0`
  (params (NewParam :type Boolean))
  (`Timeline|Timeline_0`))

(fn `NewFunction_0`)

(fn `UserConstructionScript`)