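; BP_BillboardActor is a test billboard actor whose Cube mesh toggles between its original material and a highlight ClickMaterial.
; On BeginPlay it caches the original material, then, if player controller 0 is valid, enables input and applies DefaultMesh.
; Left mouse presses alternate through a FlipFlop into SetSelected, which swaps the material.
; No hit test is made, so the toggle ignores what the cursor is over.
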(event `self.ReceiveBeginPlay`
  (bind _returnvalue (`GameplayStatics.GetPlayerController` 0))
  (set `self.CurrentMaterial` (`PrimitiveComponent.GetMaterial` (`self.Cube`) 0))
  (`/Engine/EditorBlueprintResources/StandardMacros.IsValid` _returnvalue
    (:`Is Valid`
      (`self.EnableInput` _returnvalue)
      (`StaticMeshComponent.SetStaticMesh` (`self.Cube`) (`self.DefaultMesh`)))))

(event `Key|LeftMouseButton`
  (params (Key :type "Key Structure"))
  (:`Pressed`
    (`/Engine/EditorBlueprintResources/StandardMacros.FlipFlop`
      (:`A`
        (`self.SetSelected` true))
      (:`B`
        (`self.SetSelected` false)))))

(fn `SetSelected`
  (params (Selected :type Boolean))
  (bind _cube (`self.Cube`))
  (if Selected
    (`PrimitiveComponent.SetMaterial` _cube 0 (`self.ClickMaterial`))
    (else
      (`PrimitiveComponent.SetMaterial` _cube 0 (`self.CurrentMaterial`)))))

(fn `UserConstructionScript`)